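; AI controller for the patrolling Patrol_BP pawn, which runs Patrol_BehaviorTree and reacts to AI Perception sight updates.
; Seeing the player sets it as the blackboard target, raises walk speed to sprint and flags IsFoundAI.
; Losing sight clears the target and investigation flag and stores the stimulus location as the next path point.
; UpdateTimelineStopContinue, run at BeginPlay, writes whether pawn and player share a timeline to the blackboard.
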(event OnTargetPerceptionUpdated(AIPerception)
  (params (Actor :type Actor%20Object%20Reference) (Stimulus :type AI%20Stimulus%20Structure))
  (bind _returnvalue (Class|AIPerceptionSystem|GetSenseClassforStimulus Stimulus))
  (CallFunction|HandleSense (Utilities|GetClassDisplayName _returnvalue) Stimulus Actor))

(event EventBeginPlay
  (AI|RunBehaviorTree "/Game/Content/Knight/Patrol_BehaviorTree.Patrol_BehaviorTree")
  (CallFunction|UpdateTimelineStopContinue))

(event EventTick
  (params (DeltaSeconds :type Float%20%28single-precision%29)))

(fn ConstructionScript)

(fn HandleSense
  (params (Selection :type String) (Stimulus :type AI%20Stimulus%20Structure) (SensedActor :type Actor%20Object%20Reference))
  (switch string Selection
    (:AISense_Sight
      (AI|Components|Blackboard|SetValueasBool (Variables|Default|GetBlackboard) (Utilities|Name|MakeLiteralName "isInvestigating") (.bsuccessfullysensed Stimulus))
      (if (.bsuccessfullysensed Stimulus)
        (if (== SensedActor (Game|GetPlayerCharacter 0))
          (AI|Components|Blackboard|SetValueasObject (Variables|Default|GetBlackboard) (Utilities|Name|MakeLiteralName "TargetLocationActor") SensedActor)
          (bind _aspatrol_bp (Utilities|Casting|CastToPatrol_BP (Pawn|GetControlledPawn)))
          (Variables|/Script/Engine.CharacterMovementComponent|SetMaxWalkSpeed (Variables|/Script/Engine.Character|GetCharacterMovement _aspatrol_bp) (Variables|/Game/Content/Knight/Patrol_BP.Patrol_BP_C|GetSprintSpeed _aspatrol_bp))
          (Variables|Default|SetisFoundAI true))
        (else
          (AI|Components|Blackboard|SetValueasVector (Variables|Default|GetBlackboard) (Utilities|Name|MakeLiteralName "NextPathPointVector") (.stimuluslocation Stimulus))
          (AI|Components|Blackboard|SetValueasObject (Variables|Default|GetBlackboard) (Utilities|Name|MakeLiteralName "TargetLocationActor") 0))))))

(fn UpdateTimelineStopContinue
  (bind _aspatrol_bp (Utilities|Casting|CastToPatrol_BP (Pawn|GetControlledPawn)))
  (bind _asthird_person_character (Utilities|Casting|CastToThirdPersonCharacter (Game|GetPlayerCharacter 0)))
  (AI|Components|Blackboard|SetValueasBool (Variables|Default|GetBlackboard) (Utilities|Name|MakeLiteralName "isSameTimeline") (Math|Boolean|Equal(Boolean) (Variables|/Game/Content/Knight/Patrol_BP.Patrol_BP_C|GetisCurrentTimeline _aspatrol_bp) (Variables|/Game/ThirdPersonBP/Blueprints/ThirdPersonCharacter.ThirdPersonCharacter_C|GetisCurrentTimeline _asthird_person_character)))
  (return (Math|Boolean|Equal(Boolean) (Variables|/Game/Content/Knight/Patrol_BP.Patrol_BP_C|GetisCurrentTimeline _aspatrol_bp) (Variables|/Game/ThirdPersonBP/Blueprints/ThirdPersonCharacter.ThirdPersonCharacter_C|GetisCurrentTimeline _asthird_person_character))))